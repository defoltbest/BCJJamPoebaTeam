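; Player character Blueprint with camera-relative movement, mouse look, mouse-wheel spring arm zoom, double jump, dash and hide.
; Jump launches the character through a DoN node limited to two uses, reset on landing.
; Grounded-only dash locks move input, then uses timed delays around a forward LaunchCharacter and clears its cooldown flag afterward.
; Hide toggles a flag that blocks move input; its cooldown flag resets immediately, with no delay.
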(event `InputAxis|turn`
  (params (AxisValue :type "Float (single-precision)"))
  ;[1 1 1] Мышь делает вращать
  (`self.AddControllerYawInput` AxisValue))

(event `self.ReceiveTick`
  (params (DeltaSeconds :type "Float (single-precision)")))

(event `InputAxis|Up`
  (params (AxisValue :type "Float (single-precision)"))
  ;[1 1 1] Мышь делает вращать
  (`self.AddControllerPitchInput` AxisValue))

(event `InputAction|Jump`
  (params (Key :type "Key Structure"))
  (:`Pressed`
    (`/Engine/EditorBlueprintResources/StandardMacros.Do N` 2 :!label _label
      (:`Exit`
        (`self.LaunchCharacter` (`KismetMathLibrary.MakeVector` 0.0 0.0 (`CharacterMovementComponent.JumpZVelocity` (`self.CharacterMovement`))))))))

(event `self.OnLanded`
  (params (Hit :type "HitResult Structure (by ref)"))
  (goto _label :!via `Reset`))

(event `InputAxis|MoveForward`
  (params (AxisValue :type "Float (single-precision)"))
  (bind (_returnvalue_roll _returnvalue_pitch _returnvalue_yaw) (`KismetMathLibrary.BreakRotator` (`self.GetControlRotation`)))
  ;[1 1 1] ходим по оси
  (`self.AddMovementInput` (`KismetMathLibrary.GetForwardVector` (`KismetMathLibrary.MakeRotator` 0.0 0.0 _returnvalue_yaw)) AxisValue))

(event `InputAxis|MoveRight`
  (params (AxisValue :type "Float (single-precision)"))
  (bind (_returnvalue_roll _returnvalue_pitch _returnvalue_yaw) (`KismetMathLibrary.BreakRotator` (`self.GetControlRotation`)))
  ;[1 1 1] ходим по оси
  (`self.AddMovementInput` (`KismetMathLibrary.GetRightVector` (`KismetMathLibrary.MakeRotator` 0.0 0.0 _returnvalue_yaw)) AxisValue))

(event `InputAction|Dash`
  (params (Key :type "Key Structure"))
  ;[1 1 1] ДэшОчка
  (:`Pressed`
    (if (`NavMovementComponent.IsFalling` (`self.CharacterMovement`))
      (`KismetSystemLibrary.PrintString` "Слышь бля, не лети")
      (elif (`self.Can dash?`)
        (set `self.Dash` true)
        (`Controller.SetIgnoreMoveInput` (`self.GetController`) true)
        (set `self.Can dash?` false)
        (`KismetSystemLibrary.Delay` 0.2)
        (`self.LaunchCharacter` (* (`self.GetActorForwardVector`) 3000.0) true true)
        (`KismetSystemLibrary.Delay` 0.3)
        (set `self.Dash` false)
        (set `self.Can dash?` true)
        (`Controller.SetIgnoreMoveInput` (`self.GetController`) false)
        (else
          (`KismetSystemLibrary.PrintString` "Dash CoolDown"))))))

(event `InputAction|Hide`
  (params (Key :type "Key Structure"))
  (bind _returnvalue (`self.GetController`))
  ;[1 1 1] Ныкаемся
  (:`Pressed`
    (if (`self.Can Hide?`)
      (if (`self.Hide`)
        (bind _output_get (set `self.Hide` false))
        (set `self.Can Hide?` false)
        (`Controller.SetIgnoreMoveInput` _returnvalue _output_get)
        (set `self.Can Hide?` true)
        (else
          (bind _output_get_2 (set `self.Hide` true))
          (set `self.Can Hide?` false)
          (`Controller.SetIgnoreMoveInput` _returnvalue _output_get_2)
          (set `self.Can Hide?` true)))
      (else
        (`KismetSystemLibrary.PrintString` "Hide CoolDown")))))

(event `Key|MouseScrollDown`
  (params (Key :type "Key Structure"))
  (bind _springarm (`self.SpringArm`))
  (:`Pressed`
    (set `SpringArmComponent.TargetArmLength` (- (`SpringArmComponent.TargetArmLength` _springarm) 10.0) _springarm)))

(event `Key|MouseScrollUp`
  (params (Key :type "Key Structure"))
  (bind _springarm (`self.SpringArm`))
  (:`Pressed`
    (set `SpringArmComponent.TargetArmLength` (+ (`SpringArmComponent.TargetArmLength` _springarm) 10.0) _springarm)))

(fn `UserConstructionScript`)