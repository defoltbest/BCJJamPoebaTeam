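; Player character Blueprint in a test folder that handles third-person movement, camera look and a dash.
; Mouse axes drive controller yaw and pitch, and movement axes move the character relative to the yaw of the control rotation.
; The Dash action launches the character along its forward vector, overriding its current velocity.
; The mouse wheel changes the spring arm length to zoom the camera, with no clamping.
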(event `InputAxis|turn`
  (params (AxisValue :type "Float (single-precision)"))
  ;[1 1 1] Мышь делает вращать
  (`self.AddControllerYawInput` AxisValue))

(event `InputAxis|Up`
  (params (AxisValue :type "Float (single-precision)"))
  ;[1 1 1] Мышь делает вращать
  (`self.AddControllerPitchInput` AxisValue))

(event `InputAxis|MoveForward`
  (params (AxisValue :type "Float (single-precision)"))
  (bind (_returnvalue_roll _returnvalue_pitch _returnvalue_yaw) (`KismetMathLibrary.BreakRotator` (`self.GetControlRotation`)))
  ;[1 1 1] ходим по оси
  (`self.AddMovementInput` (`KismetMathLibrary.GetForwardVector` (`KismetMathLibrary.MakeRotator` 0.0 0.0 _returnvalue_yaw)) AxisValue))

(event `InputAxis|MoveRight`
  (params (AxisValue :type "Float (single-precision)"))
  (bind (_returnvalue_roll _returnvalue_pitch _returnvalue_yaw) (`KismetMathLibrary.BreakRotator` (`self.GetControlRotation`)))
  ;[1 1 1] ходим по оси
  (`self.AddMovementInput` (`KismetMathLibrary.GetRightVector` (`KismetMathLibrary.MakeRotator` 0.0 0.0 _returnvalue_yaw)) AxisValue))

(event `InputAction|Dash`
  (params (Key :type "Key Structure"))
  (:`Pressed`
    (`self.LaunchCharacter` (* (`self.GetActorForwardVector`) 3000.0) true true)))

(event `Key|MouseScrollDown`
  (params (Key :type "Key Structure"))
  (bind _springarm (`self.SpringArm`))
  (:`Pressed`
    (set `SpringArmComponent.TargetArmLength` (- (`SpringArmComponent.TargetArmLength` _springarm) 10.0) _springarm)))

(event `Key|MouseScrollUp`
  (params (Key :type "Key Structure"))
  (bind _springarm (`self.SpringArm`))
  (:`Pressed`
    (set `SpringArmComponent.TargetArmLength` (+ (`SpringArmComponent.TargetArmLength` _springarm) 10.0) _springarm)))

(fn `UserConstructionScript`)